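; BP_Bed is an AI interactable bed, apparently an unfinished stub.
; Its StartInteraction event receives the interacting character and calls MoveComponentTo with no component or target connected.
; Unconnected nodes read the character's root component and the Box component's world location, but nothing feeds them into the move.
; The construction script only calls its parent, and the BeginPlay, overlap and Tick events are disabled.
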(event `/Game/AI2/UI/BPI_Interactable.Start Interaction`
  (params (`Interacting Character` :type "Actor Object Reference"))
  (`KismetSystemLibrary.MoveComponentTo` null))

(fn `UserConstructionScript`
  (`parent.UserConstructionScript`))